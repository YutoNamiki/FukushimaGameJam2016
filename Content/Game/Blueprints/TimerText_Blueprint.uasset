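; TimerText Blueprint is a countdown timer that shows whole seconds on a text render component and triggers the game end at zero.
; BeginPlay loads MaxTime, then Tick subtracts delta time and updates the floored text.
; Below zero it clamps, creates and plays a level sequence, then calls GameEndEvent after a delay equal to the play rate.
; This branch has no one-shot guard, so it re-enters on later ticks.
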(event EventBeginPlay
  (Variables|Default|SetTimer (Variables|Default|GetMaxTime)))

(event EventTick
  (params (DeltaSeconds :type Float%20%28single-precision%29))
  (bind _output_get (Variables|Default|SetTimer (- (Variables|Default|GetTimer) DeltaSeconds)))
  (if (< _output_get 0.0)
    (Variables|Default|SetTimer 0.0)
    (bind _returnvalue (Sequencer|Player|CreateLevelSequencePlayer 0))
    (Audio|Components|Audio|Play _returnvalue)
    (Utilities|FlowControl|Delay (Components|Animation|GetPlayRate _returnvalue))
    (Default|CallGameEndEvent))
  (Rendering|Components|TextRender|SetText (Variables|Default|GetTextRender) (Utilities|Text|ToText(Integer) (Math|Float|Floor (Variables|Default|GetTimer)))))

(fn ConstructionScript)